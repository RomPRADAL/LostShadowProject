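; Game mode that runs the chase between the player and a Shadow, driven by safe zone connections.
; MainLevelInit caches both characters, binds every safe zone's connection events and stores a checkpoint beside the starting zone.
; Losing a connection plays a sound, switches camera offset and starts an AI chase that speeds up on a looping timer.
; Finding one reverses this; smooth camera interpolation exists but is unwired, so offsets snap.
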(event Custom|Any%20Connection%20Found
  (bind _shadowref (Variables|Default|GetShadowRef))
  (bind _playerref (Variables|Default|GetPlayerRef))
  (Variables|Default|SetShouldChangeBoomOffset true)
  (Variables|/Script/Engine.SpringArmComponent|SetSocketOffset (Variables|/Game/Core/BP_ThirdPersonCharacter.BP_ThirdPersonCharacter_C|GetCameraBoom _playerref) (Variables|/Game/Core/BP_ThirdPersonCharacter.BP_ThirdPersonCharacter_C|GetSocketOffsetSafe _playerref))
  (bind _asaic_shadow_controller (Utilities|Casting|CastToAIC_ShadowController (AI|GetAIController _shadowref)))
  (Default|StopChase _asaic_shadow_controller)
  (Default|ResetSpeed _shadowref)
  (Utilities|Time|ClearandInvalidateTimerbyHandle (Variables|Default|GetAccelEvent)))

(event Custom|Any%20Connection%20Lost
  (bind _playerref (Variables|Default|GetPlayerRef))
  (Audio|PlaySoundatLocation "/Game/Assets/Son/SC_shadow_sound.SC_shadow_sound" "0, 0, 0" "0, 0, 0" 1.0 1.0 0.0 0 0 0 0)
  (Variables|Default|SetShouldChangeBoomOffset true)
  (Variables|/Script/Engine.SpringArmComponent|SetSocketOffset (Variables|/Game/Core/BP_ThirdPersonCharacter.BP_ThirdPersonCharacter_C|GetCameraBoom _playerref) (Variables|/Game/Core/BP_ThirdPersonCharacter.BP_ThirdPersonCharacter_C|GetSocketOffsetChase _playerref))
  (bind _asaic_shadow_controller (Utilities|Casting|CastToAIC_ShadowController (AI|GetAIController (Variables|Default|GetShadowRef))))
  (Default|BeginChase _asaic_shadow_controller)
  (bind _returnvalue (Utilities|Time|SetTimerbyEvent (delegate Custom|ShadowAccel) 2.0 true))
  (Variables|Default|SetAccelEvent _returnvalue))

(event Custom|ShadowAccel
  (bind _shadowref (Variables|Default|GetShadowRef))
  (bind _charactermovement (Variables|/Script/Engine.Character|GetCharacterMovement _shadowref))
  (bind _maxwalkspeed (Variables|/Script/Engine.CharacterMovementComponent|GetMaxWalkSpeed _charactermovement))
  (bind _returnvalue (+ _maxwalkspeed 1e+02))
  (Default|UpdateWalkSpeed _shadowref _returnvalue)
  (Development|PrintString (Utilities|String|Append "Current Walk speed : " (Utilities|String|ToString(Float) _returnvalue))))

(event Custom|MainLevelInit
  (Development|PrintString "Hello")
  (bind _returnvalue (Actor|GetActorOfClass "/Game/Core/BP_ThirdPersonCharacter.BP_ThirdPersonCharacter_C"))
  (Variables|Default|SetPlayerRef _returnvalue)
  (bind _returnvalue_2 (Actor|GetActorOfClass "/Game/Blueprint/AI/BP_Shadow.BP_Shadow_C"))
  (Variables|Default|SetShadowRef _returnvalue_2)
  (bind _outactors (Actor|GetAllActorsOfClass "/Game/Blueprint/BP_SafeZone.BP_SafeZone_C"))
  (bind _output_get (Variables|Default|SetAllSafeZones _outactors))
  (EventDispatchers|BindEventtoConnectionFound _output_get (delegate Custom|Any%20Connection%20Found))
  (EventDispatchers|BindEventtoConnectionLost _output_get (delegate Custom|Any%20Connection%20Lost))
  (for _array_element (Variables|Default|GetAllSafeZones)
    (if (Variables|/Game/Blueprint/BP_SafeZone.BP_SafeZone_C|GetStartingSafeZone _array_element)
      (Variables|Default|SetVecCheckpoint (Math|Vector|MakeVector (.x (Transformation|GetWorldLocation (Variables|/Script/Engine.Actor|GetRootComponent _array_element))) (+ (.y (Transformation|GetWorldLocation (Variables|/Script/Engine.Actor|GetRootComponent _array_element))) 1e+02) (.z (Transformation|GetWorldLocation (Variables|/Script/Engine.Actor|GetRootComponent _array_element)))))
      (Development|PrintString (Utilities|GetDisplayName _array_element)))))

(event EventBeginPlay)

(event EventTick
  (params (DeltaSeconds :type Float%20%28single-precision%29))
  ;[1 1 1] Si j'ai le temps
)

(fn ConstructionScript)