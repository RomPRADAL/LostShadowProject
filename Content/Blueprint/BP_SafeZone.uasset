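; BP_SafeZone is a safe zone actor that links to the player and serves as a checkpoint.
; Entering AreaOfEffect sets BPCSafeZone online, shows the cable, signals the connection and saves an offset checkpoint in the game mode; leaving reverses the connection.
; Leaving SlowArea slows the player, while re-entering it or exiting AreaOfEffect restores normal speed.
; While online, Tick moves PlayerLoc to the player, presumably as the cable's endpoint.
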(event OnComponentBeginOverlap(AreaOfEffect)
  (params (OverlappedComponent :type Primitive%20Component%20Object%20Reference) (OtherActor :type Actor%20Object%20Reference) (OtherComp :type Primitive%20Component%20Object%20Reference) (OtherBodyIndex :type Integer) (bFromSweep :type Boolean) (SweepResult :type Hit%20Result%20Structure%20%28by%20ref%29))
  (bind _returnvalue (Transformation|GetActorLocation))
  (Utilities|Casting|CastToBP_ThirdPersonCharacter OtherActor)
  (Development|PrintString "ConnectionFound")
  (Variables|/Game/Blueprint/Component/BPC_SafeZone.BPC_SafeZone_C|SetIsOnline (Variables|Default|GetBPC_SafeZone) true)
  (Development|SetHiddeninGame (Variables|Default|GetCable) false false)
  (Default|CallConnectionFound)
  (bind _asbp_lost_shadow_game_mode (Utilities|Casting|CastToBP_LostShadowGameMode (Game|GetGameMode)))
  (Variables|/Game/Core/BP_LostShadowGameMode.BP_LostShadowGameMode_C|SetVecCheckpoint _asbp_lost_shadow_game_mode (Math|Vector|MakeVector (.x _returnvalue) (+ (.y _returnvalue) 1e+02) (+ (.z _returnvalue) 1.2e+02)))
  (Development|PrintString "New Checkpoint set"))

(event OnComponentEndOverlap(AreaOfEffect)
  (params (OverlappedComponent :type Primitive%20Component%20Object%20Reference) (OtherActor :type Actor%20Object%20Reference) (OtherComp :type Primitive%20Component%20Object%20Reference) (OtherBodyIndex :type Integer))
  (bind _asbp_third_person_character (Utilities|Casting|CastToBP_ThirdPersonCharacter OtherActor))
  (Development|PrintString "ConnectionLost")
  (Variables|/Script/Engine.CharacterMovementComponent|SetMaxWalkSpeed (Variables|/Script/Engine.Character|GetCharacterMovement _asbp_third_person_character) (Variables|/Game/Core/BP_ThirdPersonCharacter.BP_ThirdPersonCharacter_C|GetRegularWalkSpeed _asbp_third_person_character))
  (Variables|/Game/Blueprint/Component/BPC_SafeZone.BPC_SafeZone_C|SetIsOnline (Variables|Default|GetBPC_SafeZone) false)
  (Development|SetHiddeninGame (Variables|Default|GetCable) true false)
  (Default|CallConnectionLost))

(event OnComponentBeginOverlap(SlowArea)
  (params (OverlappedComponent :type Primitive%20Component%20Object%20Reference) (OtherActor :type Actor%20Object%20Reference) (OtherComp :type Primitive%20Component%20Object%20Reference) (OtherBodyIndex :type Integer) (bFromSweep :type Boolean) (SweepResult :type Hit%20Result%20Structure%20%28by%20ref%29))
  (bind _asbp_third_person_character (Utilities|Casting|CastToBP_ThirdPersonCharacter OtherActor))
  (Variables|/Script/Engine.CharacterMovementComponent|SetMaxWalkSpeed (Variables|/Script/Engine.Character|GetCharacterMovement _asbp_third_person_character) (Variables|/Game/Core/BP_ThirdPersonCharacter.BP_ThirdPersonCharacter_C|GetRegularWalkSpeed _asbp_third_person_character)))

(event OnComponentEndOverlap(SlowArea)
  (params (OverlappedComponent :type Primitive%20Component%20Object%20Reference) (OtherActor :type Actor%20Object%20Reference) (OtherComp :type Primitive%20Component%20Object%20Reference) (OtherBodyIndex :type Integer))
  (bind _asbp_third_person_character (Utilities|Casting|CastToBP_ThirdPersonCharacter OtherActor))
  (Variables|/Script/Engine.CharacterMovementComponent|SetMaxWalkSpeed (Variables|/Script/Engine.Character|GetCharacterMovement _asbp_third_person_character) (Variables|/Game/Core/BP_ThirdPersonCharacter.BP_ThirdPersonCharacter_C|GetSlowedWalkSpeed _asbp_third_person_character)))

(event EventBeginPlay
  (bind _returnvalue (Actor|GetActorOfClass "/Game/Core/BP_ThirdPersonCharacter.BP_ThirdPersonCharacter_C"))
  (Variables|Default|SetPlayerRef _returnvalue)
  (bind _returnvalue_2 (Actor|GetActorOfClass "/Game/Blueprint/AI/BP_Shadow.BP_Shadow_C"))
  (bind _output_get (Variables|Default|SetShadowRef _returnvalue_2)))

(event EventTick
  (params (DeltaSeconds :type Float%20%28single-precision%29))
  (if (Variables|/Game/Blueprint/Component/BPC_SafeZone.BPC_SafeZone_C|GetIsOnline (Variables|Default|GetBPC_SafeZone))
    (Transformation|SetWorldLocation (Variables|Default|GetPlayerLoc) (Transformation|GetWorldLocation (Variables|/Script/Engine.Actor|GetRootComponent (Variables|Default|GetPlayerRef))) false false)))

(fn ConstructionScript)